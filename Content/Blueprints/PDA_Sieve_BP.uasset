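; PDA_Sieve is a Sieve of Eratosthenes that finds and counts primes up to a given limit.
; Init fills a half-sized bool array representing only odd numbers, then RunSieve clears odd multiples of each factor up to the square root, using SieveCalc for loop bounds.
; ValidateResults compares the count against known totals in PrimeCounts.
; ClearBit's parity check is disconnected, and the inner loop calls a placeholder EmptyTest.
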(fn Init
  (params (Limit :type Integer))
  (bind _output_get (Variables|Default|SetsieveSize Limit))
  (Utilities|Array|Resize (Variables|Default|GetbitArray) (/ (+ _output_get 1) 2))
  (LocalVariables|SetArrayLength (- (Utilities|Array|Length (Variables|Default|GetbitArray)) 1))
  (for _index (range 0 (LocalVariables|GetArrayLength))
    (Utilities|Array|SetArrayElem (Variables|Default|GetbitArray) _index true)))

(fn ValidateResults
  (if (Utilities|Map|Contains (Variables|Default|GetPrimeCounts) (Variables|Default|GetsieveSize))
    (return (== (CallFunction|CountPrimes) (.Value (Utilities|Map|Find (Variables|Default|GetPrimeCounts) (Variables|Default|GetsieveSize)))))
    (else
      (return false))))

(fn CountPrimes
  (for _array_element (Variables|Default|GetbitArray)
    (if _array_element
      (Math|Integer|IncrementInt (LocalVariables|Getcount))))
  (return (LocalVariables|Getcount)))

(fn GetBit
  (params (Index :type Integer))
  (if (== (Math|Integer|%(Integer) Index 2) 0)
    (return false)
    (else
      (return (Utilities|Array|Get(acopy) (Variables|Default|GetbitArray) (/ Index 2))))))

(fn ClearBit
  (params (Index :type Integer))
  (Utilities|Array|SetArrayElem (Variables|Default|GetbitArray) (/ Index 2) false))

(fn RunSieve
  (LocalVariables|Setq (Math|Float|Round (Math|Float|Sqrt (Math|Conversions|ToFloat(Integer) (Variables|Default|GetsieveSize)))))
  (while (< (LocalVariables|Getfactor) (LocalVariables|Getq))
    (bind _index (Utilities|FlowControl|ForLoopwithBreak (LocalVariables|Getfactor) (Variables|Default|GetsieveSize) :!label _label)
      (:LoopBody
        (bind _bitvalue (CallFunction|GetBit _index))
        (if _bitvalue
          (LocalVariables|Setfactor _index)
          (goto _label Break)))
      (:Completed
        (LocalVariables|SetRun2 (CallFunction|SieveCalc (LocalVariables|Getfactor)))
        (LocalVariables|Setf2 (* (LocalVariables|Getfactor) 2))
        (LocalVariables|Setf3 (* (LocalVariables|Getfactor) 3))
        (for _index_2 (range 0 (LocalVariables|GetRun2))
          (CallFunction|ClearBit (+ (* _index_2 (LocalVariables|Getf2)) (LocalVariables|Getf3)))
          (CallFunction|EmptyTest))
        (LocalVariables|Setfactor (+ (LocalVariables|Getfactor) 2))))))

(fn EmptyTest
  (LocalVariables|SetNewLocalVar_0 0))

(fn SieveCalc
  (params (A :type Integer))
  (return (/ (- (Variables|Default|GetsieveSize) (* A 3)) (* A 2))))