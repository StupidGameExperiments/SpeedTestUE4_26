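; Blueprint prime sieve (Sieve of Eratosthenes), marked OLD by its name, that flags primes up to a given limit.
; Init sizes a boolean array holding only odd numbers, halving storage, and sets every entry true.
; RunSieve finds the next set factor up to the square root, then clears its odd multiples starting at three times the factor.
; GetBit and ClearBit map numbers to half-indices; EmptyTest is an unused stub.
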(fn ClearBit
  (params (Index :type Integer))
  (if (not (== (Math|Integer|%(Integer) Index 2) 0))
    (Utilities|Array|SetArrayElem (Variables|Default|GetbitArray) (/ Index 2) false)))

(fn EmptyTest
  (LocalVariables|SetNewLocalVar_0 0))

(fn GetBit
  (params (Index :type Integer))
  (if (== (Math|Integer|%(Integer) Index 2) 0)
    (return false)
    (else
      (return (Utilities|Array|Get(acopy) (Variables|Default|GetbitArray) (/ Index 2))))))

(fn Init
  (params (Limit :type Integer))
  (bind _output_get (Variables|Default|SetsieveSize Limit))
  (Utilities|Array|Resize (Variables|Default|GetbitArray) (/ (+ _output_get 1) 2))
  (for (_ _array_index) (Variables|Default|GetbitArray)
    (Utilities|Array|SetArrayElem (Variables|Default|GetbitArray) _array_index true)))

(fn RunSieve
  (LocalVariables|Setq (Math|Float|Round (Math|Float|Sqrt (Math|Conversions|ToFloat(Integer) (Variables|Default|GetsieveSize)))))
  (while (< (LocalVariables|Getfactor) (LocalVariables|Getq))
    (bind _index (Utilities|FlowControl|ForLoopwithBreak (LocalVariables|Getfactor) (Variables|Default|GetsieveSize) :!label _label)
      (:LoopBody
        (bind _bitvalue (CallFunction|GetBit _index))
        (if _bitvalue
          (LocalVariables|Setfactor _index)
          (goto _label Break)))
      (:Completed
        (bind _index_2 (Utilities|FlowControl|ForLoopwithBreak 0 (/ (- (Variables|Default|GetsieveSize) (* (LocalVariables|Getfactor) 3)) (* (LocalVariables|Getfactor) 2)))
          (:LoopBody
            (CallFunction|ClearBit (+ (* _index_2 (* (LocalVariables|Getfactor) 2)) (* (LocalVariables|Getfactor) 3))))
          (:Completed
            (LocalVariables|Setfactor (+ (LocalVariables|Getfactor) 2))))))))